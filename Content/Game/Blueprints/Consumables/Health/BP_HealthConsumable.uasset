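; BP_HealthConsumable is a health pickup that heals the actor collecting it.
; It overrides PickUpItem, calling the parent version and then a DoOnce gate so the heal logic runs once.
; If the target has a BP_HealthComponent, it calls Heal with the ConsumableData amount and itself as instigator, then calls OnItemPickedUp.
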(fn `PickUpItem`
  (params (TargetActor :type "Actor Object Reference"))
  (bind _returnvalue (`self.GetComponentByClass` TargetActor "/Game/Game/Blueprints/Components/BP_HealthComponent.BP_HealthComponent_C"))
  (`parent.PickUpItem` TargetActor)
  (`/Engine/EditorBlueprintResources/StandardMacros.DoOnce` false
    (:`Completed`
      (`/Engine/EditorBlueprintResources/StandardMacros.IsValid` _returnvalue
        (:`Is Valid`
          (`/Game/Game/Blueprints/Components/BP_HealthComponent.Heal` _returnvalue (`/Game/Game/Blueprints/Consumables/DA_Consumable.Amount` (`self.ConsumableData`)) self)
          (`self.OnItemPickedUp`))))))

(fn `UserConstructionScript`
  (`parent.UserConstructionScript`))