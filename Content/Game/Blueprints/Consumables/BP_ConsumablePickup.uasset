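; BP_ConsumablePickup is a base pickup actor for consumables, taking its sprite and hint text from ConsumableData.
; Collision overlaps register or unregister it with actors implementing BPI_Interactor and toggle the hint text.
; Interact forwards the interacting actor to PickUpItem, an empty function that child Blueprints specialize.
; A separate OnItemPickedUp event destroys the actor.
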(event `self.ReceiveBeginPlay`
  (`PaperSpriteComponent.SetSprite` (`self.Sprite`) (`/Game/Game/Blueprints/Consumables/DA_Consumable.Icon` (`self.ConsumableData`)))
  (`self.HideHintText`)
  (`TextRenderComponent.K2_SetText` (`self.HintTextRender`) (`KismetTextLibrary.Conv_StringToText` (`/Game/Game/Blueprints/Consumables/DA_Consumable.Name` (`self.ConsumableData`)))))

(event `self.Collision.OnComponentBeginOverlap`
  (params (OverlappedComponent :type "PrimitiveComponent Object Reference") (OtherActor :type "Actor Object Reference") (OtherComp :type "PrimitiveComponent Object Reference") (OtherBodyIndex :type Integer) (bFromSweep :type Boolean) (SweepResult :type "HitResult Structure (by ref)"))
  (bind _asbpi_interactor (cast `/Game/Game/Blueprints/Interactions/BPI_Interactor` OtherActor))
  (`/Game/Game/Blueprints/Interactions/BPI_Interactor.OnInteractionEnable` _asbpi_interactor self)
  (`self.ShowHintText`))

(event `self.Collision.OnComponentEndOverlap`
  (params (OverlappedComponent :type "PrimitiveComponent Object Reference") (OtherActor :type "Actor Object Reference") (OtherComp :type "PrimitiveComponent Object Reference") (OtherBodyIndex :type Integer))
  (bind _asbpi_interactor (cast `/Game/Game/Blueprints/Interactions/BPI_Interactor` OtherActor))
  (`/Game/Game/Blueprints/Interactions/BPI_Interactor.OnInteractionDisable` _asbpi_interactor self)
  (`self.HideHintText`))

(event `/Game/Game/Blueprints/Interactions/BPI_Interactable.Interact`
  (params (`Interacting Actor` :type "Actor Object Reference"))
  (`self.PickUpItem` `Interacting Actor`))

(event `OnItemPickedUp`
  (`self.K2_DestroyActor`))

(fn `GetName`
  (returns (Name :type String))
  (return (`/Game/Game/Blueprints/Consumables/DA_Consumable.Name` (`self.ConsumableData`))))

(fn `HideHintText`
  (`SceneComponent.SetVisibility` (`self.HintTextRender`) false true))

(fn `PickUpItem`
  (params (TargetActor :type "Actor Object Reference"))
  ; Specializations in children actors
)

(fn `ShowHintText`
  (`SceneComponent.SetVisibility` (`self.HintTextRender`) true true))

(fn `UserConstructionScript`)