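; BP_KeyConsumable is a key pickup that adds its KeyCode to the key inventory of the actor that picks it up.
; It overrides PickUpItem, runs the parent logic, then passes a DoOnce gate and looks up a BP_KeysInventory component on the target.
; OnItemPickedUp fires only when AddKey succeeds, but the gate closes even on failure, with no reset.
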(fn `PickUpItem`
  (params (TargetActor :type "Actor Object Reference"))
  (bind _returnvalue (`self.GetComponentByClass` TargetActor "/Game/Game/Blueprints/Components/BP_KeysInventory.BP_KeysInventory_C"))
  (`parent.PickUpItem` TargetActor)
  (`/Engine/EditorBlueprintResources/StandardMacros.DoOnce` false
    (:`Completed`
      (`/Engine/EditorBlueprintResources/StandardMacros.IsValid` _returnvalue
        (:`Is Valid`
          (bind _badded (`/Game/Game/Blueprints/Components/BP_KeysInventory.AddKey` _returnvalue (`self.KeyCode`)))
          (if _badded
            (`self.OnItemPickedUp`)))))))

(fn `UserConstructionScript`
  (`parent.UserConstructionScript`))