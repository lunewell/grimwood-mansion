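; Key inventory component that stores a capped list of key codes.
; AddKey fails when the list is full, otherwise adds uniquely and returns true, notifying even for duplicates.
; RemoveKey checks presence with a linear search, then passes the key code to RemoveIndex as the array index.
; Both changes fire events that relay the key code through OnKeyAddedD and OnKeyRemovedD dispatchers.
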(event `OnKeyAdded`
  (params (KeyCode :type Integer))
  (`self.OnKeyAdded_D` KeyCode))

(event `OnKeyRemoved`
  (params (KeyCode :type Integer))
  (`self.OnKeyRemoved_D` KeyCode))

(fn `AddKey`
  (params (KeyCode :type "Integer (by ref)"))
  (returns (bAdded :type Boolean))
  (bind _bisfull (`self.IsInventoryFull`))
  (if _bisfull
    (return false)
    (else
      (`KismetArrayLibrary.Array_AddUnique` (`self.keys`) KeyCode)
      (`self.OnKeyAdded` KeyCode)
      (return true))))

(fn `IsInventoryFull`
  (returns (bIsFull :type Boolean))
  (return (>= (`KismetArrayLibrary.Array_Length` (`self.keys`)) (`self.MaxKeysNumber`))))

(fn `IsKeyPresent`
  (params (KeyCode :type Integer))
  (returns (bIsPresent :type Boolean))
  (for _array_element (`self.keys`)
    (if (== KeyCode _array_element)
      (return true)))
  (return false))

(fn `RemoveKey`
  (params (KeyCode :type Integer))
  (returns (bFound :type Boolean))
  (bind _bispresent (`self.IsKeyPresent` KeyCode))
  (if _bispresent
    (`KismetArrayLibrary.Array_Remove` (`self.keys`) KeyCode)
    (`self.OnKeyRemoved` KeyCode))
  (return _bispresent))