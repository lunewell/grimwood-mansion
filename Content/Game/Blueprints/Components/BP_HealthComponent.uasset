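; Health component that tracks current health, invulnerability and death, broadcasting changed, damaged, healed and death events.
; ApplyDamage adds a signed amount floored at zero and Heal caps at max, both routing through OnHealthChanged.
; UpdateDeathState runs after that broadcast, so the death check reads the prior flag; actors that cannot die refill instead.
; GetHealthPercent is empty, and SetInvulnerable copies its argument straight into CanTakeDamage, inverting its meaning.
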(event `OnHealthChanged`
  (params (`New Value` :type "Float (double-precision)") (`Old Value` :type "Float (double-precision)") (Instigator :type "Actor Object Reference (by ref)") (`Is Damage` :type Boolean))
  (`self.OnHealthChanged_D` 0.0 `New Value` Instigator (- `Old Value` `New Value`) `Is Damage`)
  (if `Is Damage`
    (`self.OnDamaged_D` Instigator `Old Value` `New Value`)
    (bind _is_dead (`self.IsDead`))
    (if _is_dead
      (`self.OnDeath_D` `Old Value` Instigator))
    (else
      (`self.OnHealed_D` Instigator `Old Value` `New Value`))))

(fn `ApplyDamage`
  (params (Amount :type "Float (double-precision)") (Instigator :type "Actor Object Reference"))
  (if (`self.bCanTakeDamage`)
    (set `self.previousHealth` (`self.currentHealth`))
    (bind _output_get (set `self.currentHealth` (`KismetMathLibrary.FMax` (+ Amount (`self.currentHealth`)))))
    (`self.OnHealthChanged` _output_get (`self.previousHealth`) Instigator true)
    (`self.UpdateDeathState`)))

(fn `GetHealthPercent`)

(fn `Heal`
  (params (Amount :type "Float (double-precision)") (Instigator :type "Actor Object Reference"))
  (set `self.previousHealth` (`self.currentHealth`))
  (bind _output_get (set `self.currentHealth` (`KismetMathLibrary.FMin` (`self.MaxHealth`) (+ Amount (`self.currentHealth`)))))
  (`self.OnHealthChanged` _output_get (`self.previousHealth`) Instigator))

(fn `IsDead`
  (returns (`Is Dead` :type Boolean))
  (return (`self.bIsDead`)))

(fn `SetInvulnerable`
  (params (`Is Invulnerable` :type Boolean))
  (set `self.bCanTakeDamage` `Is Invulnerable`))

(fn `UpdateDeathState`
  (if (<= (`self.currentHealth`) 0.0)
    (if (`self.bCanDie`)
      (set `self.bIsDead` true)
      (else
        ; If can't die and when health is zeroed, set it to max health
        (bind _output_get (set `self.currentHealth` (`self.MaxHealth`)))
        (`self.OnHealthChanged_D` 0.0 _output_get null (`self.MaxHealth`))))))