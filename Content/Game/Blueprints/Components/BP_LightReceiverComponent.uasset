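; BP_LightReceiverComponent is a component that detects sustained light exposure and signals activation.
; While enabled, OnLightHit starts a named-function timer lasting the activation time, and OnLightOut clears it and fires an interrupted event if exposure is in progress.
; The activation event calls a dispatcher so other objects can react; the start, activated and interrupted events currently print debug strings.
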(event `OnExposureStart`
  (`KismetSystemLibrary.PrintString` "Exposure Start"))

(event `OnExposureActivated`
  (`KismetSystemLibrary.PrintString` "Exposure Activated")
  (`self.OnExposureActivated_D`))

(event `OnExposureInterrupted`
  (`KismetSystemLibrary.PrintString` "Exposure Interrupted"))

(fn `DisableLightReceiver`
  (set `self.bEnabled` false))

(fn `EnableLightReceiver`
  (set `self.bEnabled` true))

(fn `IsLightReceiverEnabled`
  (returns (IsEnabled :type Boolean))
  (return (`self.bEnabled`)))

(fn `OnLightHit`
  (bind _isenabled (`self.IsLightReceiverEnabled`))
  (if _isenabled
    (`self.StartExposure`)))

(fn `OnLightOut`
  (bind _isenabled (`self.IsLightReceiverEnabled`))
  (if _isenabled
    (`self.StopExposure`)))

(fn `StartExposure`
  (if (not (`self.bIsBeingExposed`))
    (`KismetSystemLibrary.K2_SetTimer` null (`self.TimerDelegateFuncName`) (`self.ActivationTime`))
    (set `self.bIsBeingExposed` true)
    (`self.OnExposureStart`)))

(fn `StopExposure`
  (if (`self.bIsBeingExposed`)
    (`KismetSystemLibrary.K2_ClearTimer` null (`self.TimerDelegateFuncName`))
    (set `self.bIsBeingExposed` false)
    (`self.OnExposureInterrupted`)))