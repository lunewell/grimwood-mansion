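; Flashlight scene component that aims at the mouse cursor and manages a draining, rechargeable battery.
; Each tick it yaws toward the cursor's hit point and sphere-sweeps from its tagged Paper sprite child, notifying a hit actor's BP_LightReceiverComponent, or releasing the current one.
; A looping timer drains the clamped battery; drains and recharges broadcast the new value with a threshold-based state.
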(event `self.ReceiveBeginPlay`
  (`|ExecutionSequence`
    (:`then_0`
      ; Init battery
      (set `self.currentBattery` (`self.MaxBattery`))
      (`self.DrainBatteryOverTime`))
    (:`then_1`
      ; Evaluate children refs
      (for _array_element (`self.GetChildrenComponents` true)
        (if (`self.ComponentHasTag` _array_element (`self.FlashlightComponentTag`))
          (bind _aspaper_sprite_component (cast `PaperSpriteComponent` _array_element))
          (set `self.Flashlight` _aspaper_sprite_component))))))

(event `self.ReceiveTick`
  (params (DeltaSeconds :type "Float (single-precision)"))
  (bind _hitresult (`PlayerController.GetHitResultUnderCursorByChannel` (`GameplayStatics.GetPlayerController` 0) "TraceTypeQuery1" true))
  (bind _returnvalue (`self.K2_GetComponentLocation` self))
  (bind (_returnvalue_roll _returnvalue_pitch _returnvalue_yaw) (`KismetMathLibrary.BreakRotator` (`KismetMathLibrary.FindLookAtRotation` _returnvalue (`.Location` (`GameplayStatics.BreakHitResult` _hitresult)))))
  ; Rotates the flashlight following mouse position
  (`self.K2_SetWorldLocationAndRotation` self _returnvalue (`KismetMathLibrary.MakeRotator` 0.0 0.0 _returnvalue_yaw) false false)
  ; Verify actors hit by light
  (`self.CheckTorchLightReceivers` (`.Location` (`GameplayStatics.BreakHitResult` _hitresult))))

(event `OnBatteryChanged`
  (params (`New Value` :type "Float (double-precision)") (`Old Value` :type "Float (double-precision)") (Instigator :type "Actor Object Reference"))
  ; Notify externals about battery state change
  (bind _state (`self.GetBatteryState`))
  (`self.OnBatteryChanged_D` `New Value` `Old Value` Instigator _state))

(fn `CheckTorchLightReceivers`
  (params (`Mouse Location` :type "Vector Structure"))
  ; Creates the collision sphere attached to the flashlight
  (bind (_sweepstart _sweepend) (`self.SphereTraceLimitsCalc` `Mouse Location`))
  (bind _outhit (`KismetSystemLibrary.SphereTraceSingleForObjects` :`Start` _sweepstart :`End` _sweepend :`Radius` (`self.Radius`) :`ObjectTypes` (`self.LightableClasses`) :`DrawDebugType` "ForOneFrame"))
  (bind _returnvalue (`Actor.GetComponentByClass` (`.HitActor` (`GameplayStatics.BreakHitResult` _outhit)) "/Game/Game/Blueprints/Components/BP_LightReceiverComponent.BP_LightReceiverComponent_C"))
  (`/Engine/EditorBlueprintResources/StandardMacros.IsValid` _returnvalue
    (:`Is Valid`
      (`self.HitLightReceiver` _returnvalue))
    (:`Is Not Valid`
      (`self.ReleaseLightReceiver`))))

(fn `ConsumeBatteryUnit`
  (set `self.previousBattery` (`self.currentBattery`))
  (bind _output_get (set `self.currentBattery` (`KismetMathLibrary.FMax` (- (`self.currentBattery`) (`self.BatteryConsumptionAmount`)))))
  (`self.OnBatteryChanged` _output_get (`self.previousBattery`)))

(fn `DrainBatteryOverTime`
  (`KismetSystemLibrary.K2_SetTimer` null "ConsumeBatteryUnit" (`self.BatteryConsumptionDelay`) true true 0.5))

(fn `GetBatteryState`
  (returns (State :type "/Game/Game/Blueprints/Consumables/Battery/E_BatteryState Enum"))
  (if (> (`self.currentBattery`) (`self.BatteryLowThreshold`))
    (return "NewEnumerator0")
    (elif (> (`self.currentBattery`) (`self.BatteryExtremelyLowThreshold`))
      (return "NewEnumerator1")
      (elif (> (`self.currentBattery`) 0.0)
        (return "NewEnumerator2")
        (else
          (return "NewEnumerator3"))))))

(fn `HitLightReceiver`
  (params (`Light Receiver` :type "/Game/Game/Blueprints/Components/BP_LightReceiverComponent Object Reference"))
  (bind _output_get (set `self.currentLightReceiverComp` `Light Receiver`))
  (`/Game/Game/Blueprints/Components/BP_LightReceiverComponent.OnLightHit` _output_get))

(fn `RechargeBattery`
  (params (Amount :type "Float (double-precision)") (Instigator :type "Actor Object Reference"))
  (set `self.previousBattery` (`self.currentBattery`))
  (bind _output_get (set `self.currentBattery` (`KismetMathLibrary.FMin` (`self.MaxBattery`) (+ Amount (`self.currentBattery`)))))
  (`self.OnBatteryChanged` _output_get (`self.previousBattery`) Instigator))

(fn `ReleaseLightReceiver`
  (bind _currentlightreceivercomp (`self.currentLightReceiverComp`))
  (`/Engine/EditorBlueprintResources/StandardMacros.IsValid` _currentlightreceivercomp
    (:`Is Valid`
      (`/Game/Game/Blueprints/Components/BP_LightReceiverComponent.OnLightOut` _currentlightreceivercomp)
      (set `self.currentLightReceiverComp` null))))

(fn `SphereTraceLimitsCalc`
  (params (MouseCurrentLocation :type "Vector Structure"))
  (returns (SweepStart :type "Vector Structure") (SweepEnd :type "Vector Structure"))
  (bind _sweepmultiplyfactor (`self.SweepMultiplyFactor`))
  (bind _returnvalue (`self.K2_GetComponentLocation` (`self.Flashlight`)))
  (return _returnvalue (+ (* (`KismetMathLibrary.Vector_Normal2D` (- MouseCurrentLocation (`Actor.K2_GetActorLocation` (`self.GetOwner`)))) (`KismetMathLibrary.MakeVector` _sweepmultiplyfactor _sweepmultiplyfactor)) _returnvalue)))