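; BP_Ghost_1 is a ghost mob Blueprint that tracks its own movement state each frame.
; On Tick it takes the horizontal length of the CharacterMovement nav velocity as Speed.
; When Speed is nonzero it sets IsMoving and stores the X/Y velocity as MovementDirection; nothing here clears IsMoving once the ghost stops.
; The construction script only calls its parent.
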(event `self.ReceiveTick`
  (params (DeltaSeconds :type "Float (single-precision)"))
  (bind _returnvalue (`NavMovementInterface.GetVelocityForNavMovement` (`self.CharacterMovement`)))
  (bind _output_get (set `self.Speed` (`KismetMathLibrary.VSizeXY` _returnvalue)))
  (if (!= _output_get 0.0)
    (set `self.IsMoving` true)
    (set `self.MovementDirection` (`KismetMathLibrary.MakeVector2D` (.x _returnvalue) (.y _returnvalue)))))

(fn `UserConstructionScript`
  (`parent.UserConstructionScript`))