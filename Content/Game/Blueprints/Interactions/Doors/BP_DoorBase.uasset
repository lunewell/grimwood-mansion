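; Base interactable door that opens on interaction, optionally requiring a key when locked.
; Its collision overlaps enable and disable interaction on actors implementing BPI_Interactor.
; Interact uses a DoOnce gate, removes the matching KeyCode from the interactor's BP_KeysInventory if locked, and resets the gate on failure.
; OpenDoor is an empty hook for child specializations, while OnDoorOpened marks the door open, blocking further interaction.
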(event `self.Collision.OnComponentBeginOverlap`
  (params (OverlappedComponent :type "PrimitiveComponent Object Reference") (OtherActor :type "Actor Object Reference") (OtherComp :type "PrimitiveComponent Object Reference") (OtherBodyIndex :type Integer) (bFromSweep :type Boolean) (SweepResult :type "HitResult Structure (by ref)"))
  (bind _asbpi_interactor (cast `/Game/Game/Blueprints/Interactions/BPI_Interactor` OtherActor))
  (`/Game/Game/Blueprints/Interactions/BPI_Interactor.OnInteractionEnable` _asbpi_interactor self))

(event `self.Collision.OnComponentEndOverlap`
  (params (OverlappedComponent :type "PrimitiveComponent Object Reference") (OtherActor :type "Actor Object Reference") (OtherComp :type "PrimitiveComponent Object Reference") (OtherBodyIndex :type Integer))
  (bind _asbpi_interactor (cast `/Game/Game/Blueprints/Interactions/BPI_Interactor` OtherActor))
  (`/Game/Game/Blueprints/Interactions/BPI_Interactor.OnInteractionDisable` _asbpi_interactor self))

(event `/Game/Game/Blueprints/Interactions/BPI_Interactable.Interact`
  (params (`Interacting Actor` :type "Actor Object Reference"))
  (bind _returnvalue (`self.GetComponentByClass` `Interacting Actor` "/Game/Game/Blueprints/Components/BP_KeysInventory.BP_KeysInventory_C"))
  (if (not (`self.bDoorOpened`))
    (`/Engine/EditorBlueprintResources/StandardMacros.DoOnce` false :!label _label
      (:`Completed`
        (if (`self.bLocked`)
          (`/Engine/EditorBlueprintResources/StandardMacros.IsValid` _returnvalue
            (:`Is Valid`
              (bind _bfound (`/Game/Game/Blueprints/Components/BP_KeysInventory.RemoveKey` _returnvalue (`self.KeyCode`)))
              (if _bfound
                (`self.OpenDoor`)
                (else
                  ; Key not found by given code
                  (`self.ResetInteraction`))))
            (:`Is Not Valid`
              ; Not a valid actor
              (`self.ResetInteraction`)))
          (else
            (`self.OpenDoor`)))))))

(event `ResetInteraction`
  (goto _label :!via `Reset`))

(event `OnDoorOpened`
  (set `self.bDoorOpened` true)
  (`KismetSystemLibrary.PrintString` "Door opened"))

(fn `GetName`
  (returns (Name :type String))
  (return ""))

(fn `OpenDoor`
  ; Specializations in children actors
)

(fn `UserConstructionScript`)